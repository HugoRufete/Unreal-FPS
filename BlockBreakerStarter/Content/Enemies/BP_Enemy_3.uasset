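; Enemy character that chases a seen pawn, plays an attack montage and is destroyed at zero health.
; PawnSensing triggers AI MoveTo; arrival starts the attack and a cooldown, though every sighting resets CanAttack.
; Its Collider deals random damage to any overlapping actor, independently of attack state.
; Incoming damage lowers clamped health; TakeDamage only prints debug text, and UpdateColor is an empty stub.
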(event `self.ReceiveAnyDamage`
  (params (Damage :type "Float (single-precision)") (DamageType :type "DamageType Object Reference") (InstigatedBy :type "Controller Object Reference") (DamageCauser :type "Actor Object Reference"))
  (if (not (`self.enemyDead`))
    (bind _output_get (set `self.Health` (`KismetMathLibrary.FClamp` (- (`self.Health`) Damage) 0.0 (`self.MaxHealth`))))
    (if (== _output_get 0.0)
      (`self.K2_DestroyActor`)
      (else
        (`self.TakeDamage`)))))

(event `self.PawnSensing.OnSeePawn`
  (params (Pawn :type "Pawn Object Reference"))
  (set `self.canAttack` true)
  (`|ExecutionSequence`
    (:`then_0`
      (`|AIMoveTo` self (0.0 0.0 0.0) Pawn 500.0
        (:`OnSuccess`
          (if (`self.canAttack`)
            (set `self.canAttack` false)
            (`self.PlayAnimMontage` "/Game/Enemies/Animations/Enemy_3/Enemy_3_Attack_AnimMontage.Enemy_3_Attack_AnimMontage")
            (`KismetSystemLibrary.Delay` (`self.timeBetweenAttacks`))
            (set `self.canAttack` true)))))
    (:`then_1`
      (`KismetSystemLibrary.PrintString` "Jugador Visto por el enemigo"))))

(event `self.Collider.OnComponentBeginOverlap`
  (params (OverlappedComponent :type "PrimitiveComponent Object Reference") (OtherActor :type "Actor Object Reference") (OtherComp :type "PrimitiveComponent Object Reference") (OtherBodyIndex :type Integer) (bFromSweep :type Boolean) (SweepResult :type "HitResult Structure (by ref)"))
  (`GameplayStatics.ApplyDamage` OtherActor (`KismetMathLibrary.RandomFloatInRange` 10.0 20.0) null self))

(fn `TakeDamage`
  (`KismetSystemLibrary.PrintString` "Enemigo Dañado"))

(fn `UpdateColor`)

(fn `UserConstructionScript`)