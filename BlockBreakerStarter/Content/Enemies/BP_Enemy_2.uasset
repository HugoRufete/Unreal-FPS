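; BP_Enemy_2 is a dragon-sounding enemy character that chases seen pawns, attacks, and drops a heal pickup on death.
; PawnSensing drives AIMoveTo and a montage attack with a delayed cooldown, though each sighting resets CanAttack.
; Collider overlaps apply damage to any actor.
; Incoming damage lowers clamped health; death plays montage and sound, then spawns HealObject_2 at its location, ignoring the downward trace result, and destroys itself.
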(event `self.ReceiveAnyDamage`
  (params (Damage :type "Float (single-precision)") (DamageType :type "DamageType Object Reference") (InstigatedBy :type "Controller Object Reference") (DamageCauser :type "Actor Object Reference"))
  (if (not (`self.enemyDead`))
    (bind _output_get (set `self.Health` (`KismetMathLibrary.FClamp` (- (`self.Health`) Damage) 0.0 (`self.MaxHealth`))))
    (if (== _output_get 0.0)
      (set `self.enemyDead` true)
      (`self.PlayAnimMontage` "/Game/Enemies/Animations/Enemy_2/Enemy_2_Die_AnimMontage.Enemy_2_Die_AnimMontage")
      (`GameplayStatics.PlaySound2D` "/Game/BlockBreaker/Sounds/Dragon_DeadSound.Dragon_DeadSound" 1.0 1.0 0.0 null null)
      (`ActorComponent.Deactivate` (`self.CharacterMovement`))
      (`KismetSystemLibrary.Delay` 1.3)
      (`self.DropLoot`)
      (`self.K2_DestroyActor`)
      (else
        (`self.TakeDamage`)))))

(event `self.PawnSensing.OnSeePawn`
  (params (Pawn :type "Pawn Object Reference"))
  (set `self.canAttack` true)
  (if (not (`self.enemyDead`))
    (`|ExecutionSequence`
      (:`then_0`
        (`|AIMoveTo` self (0.0 0.0 0.0) Pawn 500.0
          (:`OnSuccess`
            (if (`self.canAttack`)
              (set `self.canAttack` false)
              (`GameplayStatics.PlaySound2D` "/Game/BlockBreaker/Sounds/Dragon_Attack_2.Dragon_Attack_2" 1.0 1.0 0.0 null null)
              (`self.PlayAnimMontage` "/Game/Enemies/Animations/Enemy_2/Enemy_2_Attack_Anim_Montage.Enemy_2_Attack_Anim_Montage")
              (`KismetSystemLibrary.Delay` (`self.timeBetweenAttacks`))
              (set `self.canAttack` true)))))
      (:`then_1`
        (`KismetSystemLibrary.PrintString` "Jugador Visto por el enemigo")))))

(event `self.Collider.OnComponentBeginOverlap`
  (params (OverlappedComponent :type "PrimitiveComponent Object Reference") (OtherActor :type "Actor Object Reference") (OtherComp :type "PrimitiveComponent Object Reference") (OtherBodyIndex :type Integer) (bFromSweep :type Boolean) (SweepResult :type "HitResult Structure (by ref)"))
  (`GameplayStatics.ApplyDamage` OtherActor (`self.Damage`) null self))

(fn `DropLoot`
  (bind _returnvalue (`self.K2_GetActorLocation`))
  (`KismetSystemLibrary.LineTraceSingle` _returnvalue (- _returnvalue (0.0 0.0 200.0)) "TraceTypeQuery1" false (`|MakeArray` (`GameplayStatics.GetPlayerCharacter` 0) :!type "Actor Object Reference"))
  (`|SpawnActorFromClass` "/Game/BlockBreaker/HealObject/HealObject_2.HealObject_2_C" (`KismetMathLibrary.MakeTransform` (+ (`self.K2_GetActorLocation`) (0.0 0.0 2.5))) "Undefined" "MultiplyWithRoot" null null))

(fn `TakeDamage`
  (`KismetSystemLibrary.PrintString` "Enemigo Dañado"))

(fn `UpdateColor`)

(fn `UserConstructionScript`)