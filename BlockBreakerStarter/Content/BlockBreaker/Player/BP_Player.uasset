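; BP_Player is the first-person player character for BlockBreaker, handling axis-driven movement, look, jumping, shooting and damage.
; On BeginPlay it spawns a BP_Rifle attached to GunLocation and creates the health bar widget.
; Shooting passes a camera-forward start and end point to the equipped gun, throttled by its fire rate through a CanShoot delay.
; Damage lowers clamped health on the widget, showing the Game Over screen with UI-only input at zero.
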(event `InputAxis|Jump`
  (params (AxisValue :type "Float (single-precision)"))
  ;[1 1 1] Movemente & LookAround
  (if (> AxisValue 0.0)
    (`self.Jump`)
    (else
      (`self.StopJumping`))))

(event `self.ReceiveAnyDamage`
  (params (Damage :type "Float (single-precision)") (DamageType :type "DamageType Object Reference") (InstigatedBy :type "Controller Object Reference") (DamageCauser :type "Actor Object Reference"))
  (bind _returnvalue (`GameplayStatics.GetPlayerController` 0))
  ;[1 1 1] Damage System
  (if (not (`self.isDead?`))
    (bind _output_get (set `self.Health` (`KismetMathLibrary.FClamp` (- (`self.Health`) Damage) 0.0 (`self.MaxHealth`))))
    (bind _output_get_2 (set `/Game/BlockBreaker/UI/HealthBar_Widget.Health` _output_get (`self.HealthWidget`)))
    (if (== _output_get_2 0.0)
      (bind _returnvalue_2 (`|CreateWidget` "/Game/BlockBreaker/UI/GameOver_Widget.GameOver_Widget_C"))
      (`UserWidget.AddToViewport` _returnvalue_2 0)
      (set `PlayerController.bShowMouseCursor` true _returnvalue)
      (`WidgetBlueprintLibrary.SetInputMode_UIOnlyEx` _returnvalue null)
      (else
        (`KismetSystemLibrary.PrintString` "Recibiendo Daño")))))

(event `InputAxis|MoveForward`
  (params (AxisValue :type "Float (single-precision)"))
  ;[1 1 1] Movemente & LookAround
  (`self.AddMovementInput` (`self.GetActorForwardVector`) AxisValue))

(event `InputAxis|MoveRight`
  (params (AxisValue :type "Float (single-precision)"))
  ;[1 1 1] Movemente & LookAround
  (`self.AddMovementInput` (`self.GetActorRightVector`) AxisValue))

(event `InputAxis|Shoot`
  (params (AxisValue :type "Float (single-precision)"))
  (bind _fps_camera (`self.FPS_Camera`))
  (bind _returnvalue (`SceneComponent.K2_GetComponentLocation` _fps_camera))
  ;[1 1 1] Shoot Logic
  (if (and (== AxisValue 1.0) (`self.CanShoot`))
    (`/Game/BlockBreaker/Player/BP_BaseGun.Shoot` (`self.EquippedGun`) _returnvalue (+ _returnvalue (* (`SceneComponent.GetForwardVector` _fps_camera) (`/Game/BlockBreaker/Player/BP_BaseGun.MaxBulletDistance` (`self.EquippedGun`)))))
    (set `self.CanShoot` false)
    (`KismetSystemLibrary.Delay` (`/Game/BlockBreaker/Player/BP_BaseGun.FireRate` (`self.EquippedGun`)))
    (set `self.CanShoot` true)))

(event `InputAxis|LookHorizontal`
  (params (AxisValue :type "Float (single-precision)"))
  ;[1 1 1] Movemente & LookAround
  (`self.AddControllerYawInput` AxisValue))

(event `InputAxis|LookVertical`
  (params (AxisValue :type "Float (single-precision)"))
  ;[1 1 1] Movemente & LookAround
  (`self.AddControllerPitchInput` (* AxisValue -1.0)))

(event `self.ReceiveBeginPlay`
  ;[1 1 1] Spawn Gun On Gun Location
  (`|ExecutionSequence`
    (:`then_0`
      (bind _returnvalue (`|SpawnActorFromClass` "/Game/BlockBreaker/Player/BP_Rifle.BP_Rifle_C" (`SceneComponent.K2_GetComponentToWorld` (`self.Gun_Location`)) "Undefined" "MultiplyWithRoot" null null))
      (bind _output_get (set `self.EquippedGun` _returnvalue))
      (`self.K2_AttachToComponent` _output_get (`self.Gun_Location`) "None" "SnapToTarget" "SnapToTarget" "KeepRelative" true))
    (:`then_1`
      ;[1 1 1] Instantiate IU
      (bind _returnvalue_2 (`|CreateWidget` "/Game/BlockBreaker/UI/HealthBar_Widget.HealthBar_Widget_C"))
      (bind _output_get_2 (set `self.HealthWidget` _returnvalue_2))
      (set `/Game/BlockBreaker/UI/HealthBar_Widget.MaxHealth` (`self.MaxHealth`) _output_get_2)
      (set `/Game/BlockBreaker/UI/HealthBar_Widget.Health` (`self.Health`) _output_get_2)
      (`UserWidget.AddToViewport` _returnvalue_2 0)
      (`UserWidget.AddToViewport` _output_get_2 0))))

(fn `UserConstructionScript`)