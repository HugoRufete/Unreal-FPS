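; Enemy for BlockBreaker that chases pawns it sees and hurts actors it touches.
; PawnSensing triggers AIMoveTo toward the seen pawn, while a capsule overlap applies a random amount of damage to the other actor.
; AnyDamage lowers clamped Health unless EnemyDead is set, destroying the actor at zero and otherwise calling TakeDamage, which only prints a debug message.
; UpdateColor and the construction script are empty.
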(event `self.ReceiveAnyDamage`
  (params (Damage :type "Float (single-precision)") (DamageType :type "DamageType Object Reference") (InstigatedBy :type "Controller Object Reference") (DamageCauser :type "Actor Object Reference"))
  (if (not (`self.enemyDead?`))
    (bind _output_get (set `self.Health` (`KismetMathLibrary.FClamp` (- (`self.Health`) Damage) 0.0 (`self.MaxHealth`))))
    (if (== _output_get 0.0)
      (`self.K2_DestroyActor`)
      (else
        (`self.Take Damage` 10.0)))))

(event `self.PawnSensing.OnSeePawn`
  (params (Pawn :type "Pawn Object Reference"))
  (`|AIMoveTo` self (0.0 0.0 0.0) Pawn))

(event `self.CapsuleCollider.OnComponentBeginOverlap`
  (params (OverlappedComponent :type "PrimitiveComponent Object Reference") (OtherActor :type "Actor Object Reference") (OtherComp :type "PrimitiveComponent Object Reference") (OtherBodyIndex :type Integer) (bFromSweep :type Boolean) (SweepResult :type "HitResult Structure (by ref)"))
  (`GameplayStatics.ApplyDamage` OtherActor (`KismetMathLibrary.RandomFloatInRange` 10.0 20.0) null self))

(fn `Take Damage`
  (params (Damage :type "Float (double-precision)" :default 10.0))
  (`KismetSystemLibrary.PrintString` "Enemigo Dañado"))

(fn `UpdateColor`)

(fn `UserConstructionScript`)